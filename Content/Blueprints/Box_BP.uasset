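; Box actor that moves along the spline of a referenced track actor, starting at BeginPlay when ActiveMove is set.
; MoveActor sets the timeline's play rate from Duration and its start time from StartOffset, then plays it.
; Each update stores the track value as Alpha and snaps location and rotation to the spline at GetSplineDistancebyAlpha.
; That function holds an Alpha-to-spline-length Lerp, shown as unconnected.
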(event Custom|MoveActor
  (Components|Timeline|SetPlayRate (Variables|Default|GetMoveTimeline) (/ 1.0 (Variables|Default|GetDuration)))
  (Components|Timeline|SetNewTime (Variables|Default|GetMoveTimeline) (Variables|Default|GetStartOffset))
  (CallFunction|RunTimeline))

(event Custom|RunTimeline
  (bind _새_트랙_0 (Timeline|MoveTimeline Play)
    (:Update
      (Variables|Default|SetAlpha _새_트랙_0)
      (CallFunction|MoveAlongSpline))))

(event Custom|MoveAlongSpline
  (bind _returnvalue (|GetSplineDistancebyAlpha))
  (bind _trackref (Variables|Default|GetTrackRef))
  (bind _spline (Variables|/Game/Blueprints/Spline_BP.Spline_BP_C|GetSpline _trackref))
  (Transformation|SetActorLocationAndRotation (Spline|GetLocationatDistanceAlongSpline _spline _returnvalue "World") (Spline|GetRotationatDistanceAlongSpline _spline _returnvalue "World")))

(event EventBeginPlay
  (if (Variables|Default|GetActiveMove)
    (CallFunction|MoveActor)))

(event Collision|EventActorBeginOverlap
  (params (OtherActor :type Actor%20Object%20Reference)))

(event EventTick
  (params (DeltaSeconds :type Float%20%28single-precision%29)))

(fn ConstructionScript)